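; Projectile actor for MiniGame 2 that damages minigame pawns it hits.
; The construction script sets the projectile movement velocity from its Direction variable.
; When its sphere overlaps a BP_Minigame2Pawn other than its instigator, it subtracts one from that pawn's Health and destroys itself.
; Overlaps with the instigator or any other actor type have no effect.
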(event OnComponentBeginOverlap(Sphere1)
  (params (OverlappedComponent :type Primitive%20Component%20Object%20Reference) (OtherActor :type Actor%20Object%20Reference) (OtherComp :type Primitive%20Component%20Object%20Reference) (OtherBodyIndex :type Integer) (bFromSweep :type Boolean) (SweepResult :type Hit%20Result%20Structure%20%28by%20ref%29))
  (bind _asbp_minigame_2pawn (Utilities|Casting|CastToBP_Minigame2Pawn OtherActor))
  (if (!= _asbp_minigame_2pawn (Game|GetInstigator))
    (Variables|/Game/MiniGames/MiniGame2/BP_Minigame2Pawn.BP_Minigame2Pawn_C|SetHealth _asbp_minigame_2pawn (- (Variables|/Game/MiniGames/MiniGame2/BP_Minigame2Pawn.BP_Minigame2Pawn_C|GetHealth _asbp_minigame_2pawn) 1))
    (Actor|DestroyActor)))

(fn ConstructionScript
  (Variables|/Script/Engine.MovementComponent|SetVelocity (Variables|Default|GetProjectileMovement) (Variables|Default|GetDirection)))