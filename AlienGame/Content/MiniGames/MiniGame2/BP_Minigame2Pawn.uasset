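; Minigame 2 pawn that can act as the shooter and fire projectiles.
; On BeginPlay it scans all pawns of its class and, if none is the shooter, randomly gives the role to one of the first two found.
; Pressing Action1 on the shooter spawns a projectile just above its Arrow component, aimed along the arrow's forward direction flattened to horizontal, with the pawn as instigator.
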(event EventBeginPlay
  ;[1 1 1] Begin Play
  (|CallParentFunction)
  ;[1 1 1] Check if any one in the scene is a "shooter".
  (bind _outactors (Actor|GetAllActorsOfClass "BP_Minigame2Pawn_C"))
  (for _array_element _outactors
    (Utilities|Array|Add (Variables|Default|GetShooterArray) (Variables|BP_Minigame2Pawn_C|GetShooter _array_element)))
  ;[1 1 1] Make a random pawn the "shooter"
  (if (not (Utilities|Array|ContainsItem (Variables|Default|GetShooterArray) true))
    (Variables|Default|SetRandomInt (Math|Random|RandomIntegerinRange 0 1))
    (bind _outactors_2 (Actor|GetAllActorsOfClass "BP_Minigame2Pawn_C"))
    (for (_array_element_2 _array_index) _outactors_2
      (if (== _array_index (Variables|Default|GetRandomInt))
        (Variables|BP_Minigame2Pawn_C|SetShooter _array_element_2 true)))))

(event EventTick
  (params (DeltaSeconds :type Float%20%28single-precision%29))
  ;[1 1 1] Tick
  (|CallParentFunction DeltaSeconds))

(event Input|ActionEvents|InputActionAction1
  (params (Key :type Key%20Structure))
  (bind _arrow (Variables|Default|GetArrow))
  (bind _returnvalue (Math|Vector|GetForwardVector _arrow))
  (bind _returnvalue_2 (Transformation|GetWorldTransform _arrow))
  (bind _location (Math|Transform|BreakTransform _returnvalue_2))
  ;[1 1 1] Shoot projectile
  (:Pressed
    (if (Variables|Default|GetShooter)
      (Game|SpawnActorfromClass "/Game/MiniGames/MiniGame2/Blueprint/BP_MiniGame2_Projectile.BP_MiniGame2_Projectile_C" (Math|Transform|MakeTransform (Math|Vector|MakeVector (.x _location) (.y _location) (+ (.z _location) 5e+01)) "0, 0, 0" "0.300000,0.300000,0.300000") "Undefined" 0 (Math|Vector|MakeVector (.x _returnvalue) (.y _returnvalue) 0.0) self))))

(fn ConstructionScript
  (|CallParentFunction))