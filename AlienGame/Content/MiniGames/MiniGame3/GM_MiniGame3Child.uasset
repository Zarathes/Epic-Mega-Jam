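; Child game mode for a minigame that scores teams by how much floor area their decals cover.
; On begin play it blends between two tagged cameras, starts the game after a delay, and binds an end handler that zeroes pawn movement speed.
; Each tick it resets the team results, then fires a dense grid of downward line traces, tallying decal hits per team, a costly brute-force coverage measurement.
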(event Custom|MiniGamEnd
  ;[1 1 1] MiniGameEnd
  (bind _outactors (Actor|GetAllActorsOfClass "/Game/MiniGames/MiniGame1/BP_MiniGame1Pawn.BP_MiniGame1Pawn_C"))
  (for _array_element _outactors
    (Variables|/Script/Engine.FloatingPawnMovement|SetMaxSpeed (Variables|/Game/Blueprints/Pawns/BP_CharacterPawn.BP_CharacterPawn_C|GetFloatingPawnMovement _array_element) 0.0)))

(event Custom|PerformLineTraceGrid
  (bind _results (Variables|Default|GetResults))
  ;[1 1 1] LineTrace grid
  (bind _poly_center (Utilities|2DGridExecutionMacro 25.0 "0,0,100.000000" 100 100)
    (:Per%20Poly%20Execution
      (bind _outhit (Collision|LineTraceByChannel _poly_center (- _poly_center "0, 0,200.000000") "TraceTypeQuery1" false (Variables|Default|GetActorIgnoreArray) "None" true "(R=1.000000,G=0.000000,B=0.000000,A=1.000000)" "(R=0.000000,G=1.000000,B=0.000000,A=1.000000)" 1.0))
      (bind _asbp_mini_game_1_decal (Utilities|Casting|CastToBP_MiniGame1_Decal (.HitActor (Collision|BreakHitResult _outhit))))
      (Utilities|Map|Add _results (Variables|/Game/MiniGames/MiniGame1/Blueprints/BP_MiniGame1_Decal.BP_MiniGame1_Decal_C|GetTeam _asbp_mini_game_1_decal) (+ (.Value (Utilities|Map|Find _results (Variables|/Game/MiniGames/MiniGame1/Blueprints/BP_MiniGame1_Decal.BP_MiniGame1_Decal_C|GetTeam _asbp_mini_game_1_decal))) 1)))))

(event EventBeginPlay
  ;[1 1 1] Begin Play
  (|CallParentFunction)
  (|BlendCameraAtStart
    (:Out
      (Utilities|FlowControl|Delay 2.0)
      (CallFunction|StartGameMode)
      (EventDispatchers|AssignMiniGameEnded (delegate Custom|MiniGamEnd)))))

(event EventTick
  (params (DeltaSeconds :type Float%20%28single-precision%29))
  ;[1 1 1] Event Tick and resetting results / performing grid calc
  (|CallParentFunction DeltaSeconds)
  (CallFunction|ResetResultsMap)
  (CallFunction|PerformLineTraceGrid))

(fn ConstructionScript
  (|CallParentFunction))

(fn ResetResultsMap
  (Utilities|Map|Add (Variables|Default|GetResults) "" 0)
  (Utilities|Map|Add (Variables|Default|GetResults) "NewEnumerator1" 0))