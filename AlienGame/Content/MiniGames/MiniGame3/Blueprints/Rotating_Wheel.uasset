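; Rotating wheel hazard for MiniGame3 that spins and flings player pawns that touch it.
; Once GM_MiniGame3Child reports the game started, Tick rotates the root by a fixed, frame-rate-dependent step that grows in tiers as Seconds drops.
; Overlapping the Erew component applies a fixed upward, diagonal acceleration to the BP_CharacterPawn_Mini3 Box.
; Interpolated-spin, delay and pawn-destroy nodes are disconnected leftovers.
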(event OnComponentBeginOverlap(erew)
  (params (OverlappedComponent :type Primitive%20Component%20Object%20Reference) (OtherActor :type Actor%20Object%20Reference) (OtherComp :type Primitive%20Component%20Object%20Reference) (OtherBodyIndex :type Integer) (bFromSweep :type Boolean) (SweepResult :type Hit%20Result%20Structure%20%28by%20ref%29))
  (bind _asbp_character_pawn_mini_3 (Utilities|Casting|CastToBP_CharacterPawn_Mini3 OtherActor))
  (Physics|AddForce (Variables|/Game/Blueprints/Pawns/BP_CharacterPawn.BP_CharacterPawn_C|GetBox _asbp_character_pawn_mini_3) "1000.000000,1000.000000,2000.000000" "None" true))

(event EventBeginPlay)

(event Collision|EventActorBeginOverlap
  (params (OtherActor :type Actor%20Object%20Reference)))

(event EventTick
  (params (DeltaSeconds :type Float%20%28single-precision%29))
  (bind _defaultsceneroot (Variables|Default|GetDefaultSceneRoot))
  (bind _defaultsceneroot_2 (Variables|Default|GetDefaultSceneRoot))
  (bind _asgm_mini_game_3child (Utilities|Casting|CastToGM_MiniGame3Child (Game|GetGameMode)))
  (if (Variables|/Game/Blueprints/GameMode/GM_BaseGameMode.GM_BaseGameMode_C|GetGameStarted _asgm_mini_game_3child)
    (if (>= (Variables|/Game/Blueprints/GameMode/GM_BaseGameMode.GM_BaseGameMode_C|GetSeconds _asgm_mini_game_3child) 20)
      (Transformation|AddRelativeRotation _defaultsceneroot "0,3.000000, 0" false false)
      (elif (>= (Variables|/Game/Blueprints/GameMode/GM_BaseGameMode.GM_BaseGameMode_C|GetSeconds _asgm_mini_game_3child) 15)
        (Transformation|AddRelativeRotation _defaultsceneroot "0,5.000000, 0" false false)
        (elif (>= (Variables|/Game/Blueprints/GameMode/GM_BaseGameMode.GM_BaseGameMode_C|GetSeconds _asgm_mini_game_3child) 10)
          (Transformation|AddRelativeRotation (Variables|Default|GetDefaultSceneRoot) "0,10.000000, 0" false false)
          (elif (>= (Variables|/Game/Blueprints/GameMode/GM_BaseGameMode.GM_BaseGameMode_C|GetSeconds _asgm_mini_game_3child) 5)
            (Transformation|AddRelativeRotation _defaultsceneroot_2 "0,15.000000, 0" false false)
            (else
              (Transformation|AddRelativeRotation _defaultsceneroot_2 "0,20.000000, 0" false false))))))))

(fn ConstructionScript)