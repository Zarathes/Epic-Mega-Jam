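; Game mode for MiniGame 3 in Aliens VS Government.
; BeginPlay caches the game instance and sets Timer from the minigame duration, while Tick only calls the parent.
; A custom event clears GameStarted and signals the minigame's end.
; Disconnected leftover logic holds a widget countdown, start signal, unfinished team-based pawn possession and timer-driven game end, none of which runs.
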(event Custom|CustomEvent
  ;[1 1 1] MiniGame End event
  (Variables|Default|SetGameStarted false)
  (Default|CallMiniGameEnded))

(event EventTick
  (params (DeltaSeconds :type Float%20%28single-precision%29))
  ;[1 1 1] Update timer as soon as the game has started.
  (|CallParentFunction DeltaSeconds))

(event EventBeginPlay
  ;[1 1 1] Get Game Instance
  (|CallParentFunction)
  (bind _asinstance_aliens_vsgovernment (Utilities|Casting|CastToInstance_AliensVSGovernment (Game|GetGameInstance)))
  (Variables|Default|SetGameInstance _asinstance_aliens_vsgovernment)
  ;[1 1 1] Set Timer off Minigame Duration
  (Variables|Default|SetTimer (Math|Conversions|ToFloat(Integer) (Variables|Default|GetMiniGameDuration))))

(fn ConstructionScript
  (|CallParentFunction))