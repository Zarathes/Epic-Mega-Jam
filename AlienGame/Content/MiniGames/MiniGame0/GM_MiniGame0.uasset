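; Game mode for MiniGame0 that spawns two local players at team spawn points for an Aliens versus Government match.
; On BeginPlay it sorts TeamStart actors into per-team lists, creates both players, and teleports each pawn to a random point for its side stored in the game instance.
; It also sets each pawn's team and index, and overrides FindPlayerStart to pick a random start from the controller's team.
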(event EventBeginPlay
  ;[1 1 1] Begin Play
  (bind _asinstance_aliens_vsgovernment (Utilities|Casting|CastToInstance_AliensVSGovernment (Game|GetGameInstance)))
  (Variables|Default|SetGameInstanceRef _asinstance_aliens_vsgovernment)
  (SpawnPoint|FindAllSpawnPoints)
  (Spawning|SpawnPlayer)
  (Spawning|SpawnPlayer 1))

(fn ConstructionScript)

(fn FindAllSpawnPoints
  (bind _outactors (Actor|GetAllActorsOfClass "/Game/Blueprints/Pawns/TeamStart.TeamStart_C"))
  (for _array_element _outactors
    (switch Utilities|FlowControl|Switch|SwitchonEnum_Teams (Variables|/Game/Blueprints/Pawns/TeamStart.TeamStart_C|GetTeam _array_element)
      (:NewEnumerator0
        (Utilities|Array|Add (Variables|Default|GetAlienSpawnPoints) _array_element))
      (:NewEnumerator1
        (Utilities|Array|Add (Variables|Default|GetGovernmentSpawnPoints) _array_element))))
  (return))

(fn FindPlayerStart
  (params (Player :type Controller%20Object%20Reference) (IncomingName :type String))
  ;[1 1 1] Custom override to change player spawns
  (if (or (== (Utilities|Array|Length (Variables|Default|GetAlienSpawnPoints)) 0) (== (Utilities|Array|Length (Variables|Default|GetGovernmentSpawnPoints)) 0))
    (SpawnPoint|FindAllSpawnPoints))
  (bind _aspc_player (Utilities|Casting|CastToPC_Player Player))
  (switch Utilities|FlowControl|Switch|SwitchonEnum_Teams (Variables|/Game/Blueprints/Pawns/PlayerControllers/PC_Player.PC_Player_C|GetTeam _aspc_player)
    (:NewEnumerator0
      (return (Utilities|Array|Get(acopy) (Variables|Default|GetAlienSpawnPoints) (Math|Random|RandomIntegerinRange 0 (- (Utilities|Array|Length (Variables|Default|GetAlienSpawnPoints)) 1)))))
    (:NewEnumerator1
      (return (Utilities|Array|Get(acopy) (Variables|Default|GetGovernmentSpawnPoints) (Math|Random|RandomIntegerinRange 0 (- (Utilities|Array|Length (Variables|Default|GetGovernmentSpawnPoints)) 1)))))))

(fn FindPlayerSpawnPoint
  (params (Team :type Enum_Teams%20Enum :default "NewEnumerator0"))
  (switch Utilities|FlowControl|Switch|SwitchonEnum_Teams Team
    (:NewEnumerator0
      (return (Utilities|Array|Get(acopy) (Variables|Default|GetAlienSpawnPoints) (Math|Random|RandomIntegerinRange 0 (- (Utilities|Array|Length (Variables|Default|GetAlienSpawnPoints)) 1)))))
    (:NewEnumerator1
      (return (Utilities|Array|Get(acopy) (Variables|Default|GetGovernmentSpawnPoints) (Math|Random|RandomIntegerinRange 0 (- (Utilities|Array|Length (Variables|Default|GetGovernmentSpawnPoints)) 1)))))))

(fn SpawnPlayer
  (params (PlayerNumber :type Integer))
  (bind _gameinstanceref (Variables|Default|GetGameInstanceRef))
  (bind _playersides (Variables|/Game/Blueprints/GameInstance/Instance_AliensVSGovernment.Instance_AliensVSGovernment_C|GetPlayerSides _gameinstanceref))
  (bind _output (Utilities|Array|Get(acopy) _playersides PlayerNumber))
  (bind _returnvalue (Class|GameplayStatics|CreatePlayer PlayerNumber))
  (bind _returnvalue_2 (SpawnPoint|FindPlayerSpawnPoint _output))
  (bind _asbp_character_pawn (Utilities|Casting|CastToBP_CharacterPawn (Pawn|GetControlledPawn _returnvalue)))
  (Transformation|SetActorTransform _asbp_character_pawn (Transformation|GetActorTransform _returnvalue_2) false true)
  (Variables|/Game/Blueprints/Pawns/BP_CharacterPawn.BP_CharacterPawn_C|SetTeam _asbp_character_pawn _output)
  (Variables|/Game/Blueprints/Pawns/BP_CharacterPawn.BP_CharacterPawn_C|SetPlayerIndex _asbp_character_pawn PlayerNumber))