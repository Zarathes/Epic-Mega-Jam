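; BP_MiniGame1Pawn is the player pawn for MiniGame1 that shoots team goop onto the surface beneath it.
; Pressing Action1 runs a debug-drawn line trace from the root along its down vector against WorldStatic objects.
; On a hit, it spawns a BP_MiniGame1_Decal at the impact point with random yaw, zero initial scale and the pawn's Team.
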(event EventBeginPlay
  (|CallParentFunction) ; This node is disabled and will not be called.\nDrag off pins to build functionality.
)

(event Collision|EventActorBeginOverlap
  (params (OtherActor :type Actor%20Object%20Reference)))

(event EventTick
  (params (DeltaSeconds :type Float%20%28single-precision%29))
  (|CallParentFunction DeltaSeconds) ; This node is disabled and will not be called.\nDrag off pins to build functionality.
)

(event Input|ActionEvents|InputActionAction1
  (params (Key :type Key%20Structure))
  (bind _defaultsceneroot (Variables|Default|GetDefaultSceneRoot))
  (bind _returnvalue (Transformation|GetWorldLocation _defaultsceneroot))
  ;[1 1 1] Shoot Goop
  (:Pressed
    (bind (_outhit _returnvalue_2) (Collision|LineTraceForObjects _returnvalue (+ _returnvalue (* (* (Math|Vector|GetUpVector _defaultsceneroot) -1.0) 2000)) (Utilities|Array|MakeArray "ObjectTypeQuery1") false 0 "ForDuration"))
    (if _returnvalue_2
      (Game|SpawnActorfromClass "/Game/MiniGames/MiniGame1/Blueprints/BP_MiniGame1_Decal.BP_MiniGame1_Decal_C" (Math|Transform|MakeTransform (.Location (Collision|BreakHitResult _outhit)) (Math|Rotator|MakeRotator 0.0 0.0 (Math|Random|RandomFloatinRange 0.0 3.6e+02)) "0.000000,0.000000,0.000000") "Undefined" 0 (Variables|Default|GetTeam) 0))))

(fn ConstructionScript
  (|CallParentFunction))