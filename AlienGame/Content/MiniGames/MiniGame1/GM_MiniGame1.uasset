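; Game mode for MiniGame1 that measures how much of the play area the Aliens and Government teams each cover with decal actors.
; Every Tick it resets the per-team results map, then fires short downward visibility traces across a 100x100 grid around a fixed center.
; Each trace hitting a BP_MiniGame1_Decal increments that decal's team count.
; Counts are divided by 100 into coverage percentages and printed on screen every frame.
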(event Custom|PerformLineTraceGrid
  (bind _results (Variables|Default|GetResults))
  (bind _poly_center (Utilities|2DGridExecutionMacro 25.0 "0,0,100.000000" 100 100)
    (:Per%20Poly%20Execution
      (bind _outhit (Collision|LineTraceByChannel _poly_center (- _poly_center "0, 0,200.000000") "TraceTypeQuery1" false (Variables|Default|GetActorIgnoreArray) "None" true "(R=1.000000,G=0.000000,B=0.000000,A=1.000000)" "(R=0.000000,G=1.000000,B=0.000000,A=1.000000)" 0.1))
      (bind _asbp_mini_game_1_decal (Utilities|Casting|CastToBP_MiniGame1_Decal (.HitActor (Collision|BreakHitResult _outhit))))
      (Utilities|Map|Add _results (Variables|/Game/MiniGames/MiniGame1/Blueprints/BP_MiniGame1_Decal.BP_MiniGame1_Decal_C|GetTeam _asbp_mini_game_1_decal) (+ (.Value (Utilities|Map|Find _results (Variables|/Game/MiniGames/MiniGame1/Blueprints/BP_MiniGame1_Decal.BP_MiniGame1_Decal_C|GetTeam _asbp_mini_game_1_decal))) 1)))))

(event EventTick
  (params (DeltaSeconds :type Float%20%28single-precision%29))
  (bind _returnvalue (Utilities|Time|GetWorldDeltaSeconds))
  (bind _results (Variables|Default|GetResults))
  (CallFunction|ResetResultsMap)
  (CallFunction|PerformLineTraceGrid)
  (Development|PrintString (Utilities|String|BuildString(Integer) "" "Aliens:" (/ (.Value (Utilities|Map|Find _results "")) 100)) true true "(R=0.000000,G=0.660000,B=1.000000,A=1.000000)" _returnvalue)
  (Development|PrintString (Utilities|String|BuildString(Integer) "" "Government: " (/ (.Value (Utilities|Map|Find _results "NewEnumerator1")) 100)) true true "(R=0.000000,G=0.660000,B=1.000000,A=1.000000)" _returnvalue))

(fn ConstructionScript)

(fn ResetResultsMap
  (Utilities|Map|Add (Variables|Default|GetResults) "NewEnumerator0" 0)
  (Utilities|Map|Add (Variables|Default|GetResults) "NewEnumerator1" 0))