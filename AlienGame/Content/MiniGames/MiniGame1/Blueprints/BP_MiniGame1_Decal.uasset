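; BP_MiniGame1_Decal is a team-colored splat actor for MiniGame1, belonging to either Aliens or Government.
; The construction script picks a random mesh, sets its Color material parameter by team and randomizes yaw.
; Tick scales the actor up toward full size, simulating a fade-in.
; Shortly after BeginPlay, it flags overlapping enemy-team decals to fade out, reversing their scaling until they shrink below zero and destroy themselves.
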(event EventBeginPlay
  (Utilities|FlowControl|Delay 0.4)
  (for _array_element (Collision|GetOverlappingActors (Variables|Default|GetStaticMesh) 0 :!class /Script/Engine.PrimitiveComponent)
    (bind _asbp_mini_game_1_decal (Utilities|Casting|CastToBP_MiniGame1_Decal _array_element))
    (if (Utilities|Enum|NotEqual(Enum) (Variables|BP_MiniGame1_Decal_C|GetTeam _asbp_mini_game_1_decal) (Variables|Default|GetTeam))
      (Variables|BP_MiniGame1_Decal_C|SetFadeOut _asbp_mini_game_1_decal true)
      (Variables|BP_MiniGame1_Decal_C|SetFadeMultiplier _asbp_mini_game_1_decal -0.3))))

(event EventTick
  (params (DeltaSeconds :type Float%20%28single-precision%29))
  (bind _secondstofadein (Variables|Default|GetSecondsToFadeIn))
  (bind _returnvalue (/ 1.0 _secondstofadein))
  (if (or (Variables|Default|GetFadeOut) (not (>= (.x (Transformation|GetActorScale3D)) 1.0)))
    (Transformation|SetActorScale3D (+ (* (* (Math|Vector|MakeVector _returnvalue _returnvalue _returnvalue) DeltaSeconds) (Variables|Default|GetFadeMultiplier)) (Transformation|GetActorScale3D)))
    (if (< (.x (Transformation|GetActorScale3D)) 0.0)
      (Actor|DestroyActor))))

(fn ConstructionScript
  (bind _staticmesh (Variables|Default|GetStaticMesh))
  (Components|StaticMesh|SetStaticMesh (Variables|Default|GetStaticMesh) (Utilities|Array|Get(acopy) (Variables|Default|GetMeshOptions) (Math|Random|RandomIntegerinRange 0 (- (Utilities|Array|Length (Variables|Default|GetMeshOptions)) 1))))
  (switch Utilities|FlowControl|Switch|SwitchonEnum_Teams (Variables|Default|GetTeam)
    (:NewEnumerator0
      (Rendering|Material|SetVectorParameterValueonMaterials _staticmesh "Color" "0.420000,0.050000,0.500000"))
    (:NewEnumerator1
      (Rendering|Material|SetVectorParameterValueonMaterials _staticmesh "Color" "0.000000,0.000000,0.000000")))
  (Transformation|SetWorldRotation (Variables|Default|GetStaticMesh) (Math|Rotator|MakeRotator 0.0 0.0 (Math|Random|RandomFloatinRange 0.0 3.6e+02)) false false))