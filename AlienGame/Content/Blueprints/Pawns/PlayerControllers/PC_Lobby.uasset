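; PC_Lobby is the lobby player controller for team selection and starting a minigame in Aliens VS Government.
; Gamepad special buttons, Enter and Escape call Enter or Credits on the top-level UI_MainMenu widget.
; Left and right assign this controller a team through the cached game instance if available, while up sets a third option unchecked.
; Start launches a hard-coded minigame entry once the game instance reports players ready.
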(event EventBeginPlay
  (bind _asinstance_aliens_vsgovernment (Utilities|Casting|CastToInstance_AliensVSGovernment (Game|GetGameInstance)))
  (Variables|Default|SetGameInstance _asinstance_aliens_vsgovernment))

(event Input|ActionEvents|InputActionUIStart
  (params (Key :type Key%20Structure))
  (bind _gameinstance (Variables|Default|GetGameInstance))
  (:Pressed
    (if (Variables|/Game/Blueprints/GameInstance/Instance_AliensVSGovernment.Instance_AliensVSGovernment_C|GetPlayersReady (Variables|Default|GetGameInstance))
      (Default|StartMiniGame _gameinstance (Utilities|Array|Get(acopy) (Variables|/Game/Blueprints/GameInstance/Instance_AliensVSGovernment.Instance_AliensVSGovernment_C|GetMiniGameInformation _gameinstance) 1)))))

(event Input|ActionEvents|InputActionUIMoveLeft
  (params (Key :type Key%20Structure))
  (bind _gameinstance (Variables|Default|GetGameInstance))
  (:Pressed
    (bind _teamavailible (Default|TeamAvailable _gameinstance "NewEnumerator0"))
    (if _teamavailible
      (Default|SetPlayerConfig _gameinstance (Class|GameplayStatics|GetPlayerControllerID self) "NewEnumerator0"))))

(event Input|ActionEvents|InputActionUIMoveRight
  (params (Key :type Key%20Structure))
  (bind _gameinstance (Variables|Default|GetGameInstance))
  (:Pressed
    (bind _teamavailible (Default|TeamAvailable _gameinstance "NewEnumerator1"))
    (if _teamavailible
      (Default|SetPlayerConfig _gameinstance (Class|GameplayStatics|GetPlayerControllerID self) "NewEnumerator1"))))

(event Input|ActionEvents|InputActionUIMoveUp
  (params (Key :type Key%20Structure))
  (:Pressed
    (Default|SetPlayerConfig (Variables|Default|GetGameInstance) (Class|GameplayStatics|GetPlayerControllerID self) "NewEnumerator2")))

(event Input|KeyboardEvents|Enter
  (params (Key :type Key%20Structure))
  (:Pressed
    (bind _foundwidgets (Widget|GetAllWidgetsOfClass "/Game/Blueprints/UI/MainMenu/UI_MainMenu.UI_MainMenu_C" true))
    (Utilities|IsValid (Utilities|Array|Get(acopy) _foundwidgets)
      (:Is%20Valid
        (Default|Enter (Utilities|Array|Get(acopy) _foundwidgets))))))

(event Input|GamepadEvents|GamepadSpecialRight
  (params (Key :type Key%20Structure))
  (:Pressed
    (bind _foundwidgets (Widget|GetAllWidgetsOfClass "/Game/Blueprints/UI/MainMenu/UI_MainMenu.UI_MainMenu_C" true))
    (Utilities|IsValid (Utilities|Array|Get(acopy) _foundwidgets)
      (:Is%20Valid
        (Default|Enter (Utilities|Array|Get(acopy) _foundwidgets))))))

(event Input|GamepadEvents|GamepadSpecialLeft
  (params (Key :type Key%20Structure))
  (:Pressed
    (bind _foundwidgets (Widget|GetAllWidgetsOfClass "/Game/Blueprints/UI/MainMenu/UI_MainMenu.UI_MainMenu_C" true))
    (Default|Credits (Utilities|Array|Get(acopy) _foundwidgets))))

(event Input|KeyboardEvents|Escape
  (params (Key :type Key%20Structure))
  (:Pressed
    (bind _foundwidgets (Widget|GetAllWidgetsOfClass "/Game/Blueprints/UI/MainMenu/UI_MainMenu.UI_MainMenu_C" true))
    (Default|Credits (Utilities|Array|Get(acopy) _foundwidgets))))

(fn ConstructionScript)