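; Player pawn for Aliens vs Government that appears as either a UFO or a government car, depending on its team.
; BeginPlay reads the team from the game instance's player configuration and sets mesh, offset and lights; the Construction Script repeats this setup from the Team variable.
; Axis input drives FloatingPawnMovement along an arrow component's axes.
; Tick eases the mesh toward velocity, adds a cosine bob, and spins the UFO when idle.
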(event Custom|UpdateTickAlien
  (bind _returnvalue (Transformation|GetVelocity))
  (bind _mesh (Variables|Default|GetMesh))
  (bind _mesh_2 (Variables|Default|GetMesh))
  (bind _mesh_3 (Variables|Default|GetMesh))
  (bind _returnvalue_2 (Math|Rotator|MakeRotfromX _returnvalue))
  (bind _relativerotation (Variables|/Script/Engine.SceneComponent|GetRelativeRotation _mesh_2))
  (bind _relativelocation (Variables|/Script/Engine.SceneComponent|GetRelativeLocation _mesh))
  (bind (_roll _pitch _yaw) (Math|Rotator|BreakRotator _returnvalue_2))
  ;[1 1 1] Alien Tick
  ;[1 1 1] Face alien towards direction it is moving in
  (if (Math|Vector|NotEqual(Vector) _returnvalue "0, 0, 0" 0.0001)
    (Transformation|SetRelativeRotation _mesh_3 (Math|Interpolation|RInterpTo (Variables|/Script/Engine.SceneComponent|GetRelativeRotation _mesh_3) (Math|Rotator|MakeRotator _roll _pitch (- _yaw 9e+01)) (Utilities|Time|GetWorldDeltaSeconds) 6.0) false false)
    (else
      ;[1 1 1] Make alien rotate when not moving.
      (Transformation|SetRelativeRotation _mesh_2 (Math|Rotator|MakeRotator (.roll _relativerotation) (.pitch _relativerotation) (+ (.yaw _relativerotation) (* (Utilities|Time|GetWorldDeltaSeconds) 5e+01))) false false)))
  ;[1 1 1] Make alien wobble
  (Transformation|SetRelativeLocation (Variables|Default|GetMesh) (Math|Vector|MakeVector (.x _relativelocation) (.y _relativelocation) (+ (.z _relativelocation) (* (Math|Trig|Cos(Radians) (* (Actor|GetGameTimeSinceCreation) 6.0)) 1.0))) false false))

(event Custom|UpdateTickGovernment
  (bind _returnvalue (Transformation|GetVelocity))
  (bind _mesh (Variables|Default|GetMesh))
  (bind _mesh_2 (Variables|Default|GetMesh))
  (bind _returnvalue_2 (Math|Rotator|MakeRotfromX _returnvalue))
  (bind _relativelocation (Variables|/Script/Engine.SceneComponent|GetRelativeLocation _mesh_2))
  (bind (_roll _pitch _yaw) (Math|Rotator|BreakRotator _returnvalue_2))
  ;[1 1 1] Government Tick
  ;[1 1 1] Face car towards direction it is moving in
  (if (Math|Vector|NotEqual(Vector) _returnvalue "0, 0, 0" 0.0001)
    (Transformation|SetRelativeRotation _mesh (Math|Interpolation|RInterpTo (Variables|/Script/Engine.SceneComponent|GetRelativeRotation _mesh) (Math|Rotator|MakeRotator _roll _pitch (- _yaw 9e+01)) (Utilities|Time|GetWorldDeltaSeconds) 6.0) false false))
  (Transformation|SetRelativeLocation (Variables|Default|GetMesh) (Math|Vector|MakeVector (.x _relativelocation) (.y _relativelocation) (+ (.z _relativelocation) (* (Math|Trig|Cos(Radians) (* (Actor|GetGameTimeSinceCreation) 2e+01)) 1.0))) false false))

(event EventBeginPlay
  (bind _mesh (Variables|Default|GetMesh))
  (bind _ufolight1 (Variables|Default|GetUFOLight1))
  (bind _carlight1 (Variables|Default|GetCarLight1))
  ;[1 1 1] Set team according to player config system
  (bind _asinstance_aliens_vsgovernment (Utilities|Casting|CastToInstance_AliensVSGovernment (Game|GetGameInstance)))
  (Variables|Default|SetTeam (.Value (Utilities|Map|Find (Variables|/Game/Blueprints/GameInstance/Instance_AliensVSGovernment.Instance_AliensVSGovernment_C|GetPlayerConfiguration _asinstance_aliens_vsgovernment) (Class|GameplayStatics|GetPlayerControllerID (Game|GetPlayerController (Variables|Default|GetPlayerIndex))))))
  ;[1 1 1] Switch on team
  (switch Utilities|FlowControl|Switch|SwitchonEnum_Teams (Variables|Default|GetTeam)
    (:NewEnumerator0
      ;[1 1 1] Toggle model and offset
      (Components|StaticMesh|SetStaticMesh _mesh "/Game/Art/Alien/SM_AlienUFO.SM_AlienUFO")
      (Transformation|SetRelativeLocation _mesh "0, 0,80.000000" false false)
      ;[1 1 1] Toggle Lights
      (Rendering|SetVisibility _ufolight1 true false)
      (Rendering|SetVisibility _carlight1 false false))
    (:NewEnumerator1
      (Components|StaticMesh|SetStaticMesh _mesh "/Game/Art/Government/SM_GovernmentCarCombined.SM_GovernmentCarCombined")
      (Transformation|SetRelativeLocation _mesh "0, 0,30.000000" false false)
      (Rendering|SetVisibility _ufolight1 false false)
      (Rendering|SetVisibility _carlight1 true false))))

(event EventTick
  (params (DeltaSeconds :type Float%20%28single-precision%29))
  ;[1 1 1] Tick Events
  (switch Utilities|FlowControl|Switch|SwitchonEnum_Teams (Variables|Default|GetTeam)
    (:NewEnumerator0
      (CallFunction|UpdateTickAlien))
    (:NewEnumerator1
      (CallFunction|UpdateTickGovernment))))

(event Input|AxisEvents|InputAxisMoveX
  (params (AxisValue :type Float%20%28single-precision%29))
  ;[1 1 1] Default X & Y input
  (Class|PawnMovementComponent|AddInputVector (Variables|Default|GetFloatingPawnMovement) (* (* (Math|Vector|GetRightVector (Variables|Default|GetForwardDirectionArrow)) (Variables|Movement|GetMovementSpeed)) AxisValue) false))

(event Input|AxisEvents|InputAxisMoveY
  (params (AxisValue :type Float%20%28single-precision%29))
  ;[1 1 1] Default X & Y input
  (Class|PawnMovementComponent|AddInputVector (Variables|Default|GetFloatingPawnMovement) (* (* (Math|Vector|GetForwardVector (Variables|Default|GetForwardDirectionArrow)) (Variables|Movement|GetMovementSpeed)) AxisValue) false))

(fn ConstructionScript
  (bind _mesh (Variables|Default|GetMesh))
  (bind _ufolight1 (Variables|Default|GetUFOLight1))
  (bind _carlight1 (Variables|Default|GetCarLight1))
  ;[1 1 1] Switch on team
  (switch Utilities|FlowControl|Switch|SwitchonEnum_Teams (Variables|Default|GetTeam)
    (:NewEnumerator0
      ;[1 1 1] Toggle model and offset
      (Components|StaticMesh|SetStaticMesh _mesh "/Game/Art/Alien/SM_AlienUFO.SM_AlienUFO")
      (Transformation|SetRelativeLocation _mesh "0, 0,80.000000" false false)
      ;[1 1 1] Toggle Lights
      (Rendering|SetVisibility _ufolight1 true false)
      (Rendering|SetVisibility _carlight1 false false))
    (:NewEnumerator1
      (Components|StaticMesh|SetStaticMesh _mesh "/Game/Art/Government/SM_GovernmentCarCombined.SM_GovernmentCarCombined")
      (Transformation|SetRelativeLocation _mesh "0, 0,30.000000" false false)
      (Rendering|SetVisibility _ufolight1 false false)
      (Rendering|SetVisibility _carlight1 true false))))