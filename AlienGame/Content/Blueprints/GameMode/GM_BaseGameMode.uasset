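; Base game mode for timed two-player minigames in Aliens VS Government, handling start, countdown and end.
; StartGameMode fires the minigame-started dispatcher, then has player controllers 0 and 1 possess the BP_CharacterPawns whose Team matches their game instance config.
; Tick accumulates elapsed time while the game runs and calls EndGameMode at MiniGameDuration, which clears the running flag and fires the ended dispatcher.
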(event Custom|StartGameMode
  (bind _gameinstance (Variables|Default|GetGameInstance))
  ;[1 1 1] MiniGame Start event
  (Variables|MinigameFlow|SetGameStarted true)
  (Default|CallMiniGameStarted)
  ;[1 1 1] Posses pawns
  (bind _outactors (Actor|GetAllActorsOfClass "/Game/Blueprints/Pawns/BP_CharacterPawn.BP_CharacterPawn_C"))
  (for _array_element _outactors
    (bind _team (Default|FindPlayerConfig _gameinstance))
    (if (Utilities|Enum|Equal(Enum) _team (Variables|/Game/Blueprints/Pawns/BP_CharacterPawn.BP_CharacterPawn_C|GetTeam _array_element))
      (Pawn|Possess (Game|GetPlayerController 0) _array_element)
      (else
        (bind _team_2 (Default|FindPlayerConfig _gameinstance 1))
        (if (Utilities|Enum|Equal(Enum) _team_2 (Variables|/Game/Blueprints/Pawns/BP_CharacterPawn.BP_CharacterPawn_C|GetTeam _array_element))
          (Pawn|Possess (Game|GetPlayerController 1) _array_element))))))

(event Custom|EndGameMode
  ;[1 1 1] MiniGame End event
  (Variables|MinigameFlow|SetGameStarted false)
  (Default|CallMiniGameEnded))

(event EventTick
  (params (DeltaSeconds :type Float%20%28single-precision%29))
  ;[1 1 1] Update timer as soon as the game has started.
  (if (Variables|MinigameFlow|GetGameStarted)
    (bind _output_get (Variables|Timer|SetTimer (+ (Variables|Timer|GetTimer) DeltaSeconds)))
    (Variables|Timer|SetSeconds (Math|Float|Truncate _output_get))
    ;[1 1 1] End Game mode when time is reached
    (if (>= (Variables|Timer|GetSeconds) (Variables|MinigameFlow|GetMiniGameDuration))
      (CallFunction|EndGameMode))))

(event EventBeginPlay
  ;[1 1 1] Get Game Instance
  (bind _asinstance_aliens_vsgovernment (Utilities|Casting|CastToInstance_AliensVSGovernment (Game|GetGameInstance)))
  (Variables|Default|SetGameInstance _asinstance_aliens_vsgovernment))

(fn ConstructionScript)