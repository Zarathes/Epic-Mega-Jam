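; Lobby game mode that sets up local players and tracks whether players are ready in the Aliens VS Government game instance.
; On BeginPlay it loops creating local players with pawns until more than one exists or creation fails, printing debug strings.
; Every Tick it sets the instance's PlayersReady flag by comparing player configs against one enum value.
; Both config lookups use index 0, so only the first player's config is checked.
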(event Custom|Create%20Players
  (while (Variables|Default|GetContinue)
    (bind _returnvalue (Class|GameModeBase|GetNumPlayers))
    (Development|PrintString (Utilities|String|ToString(Integer) _returnvalue))
    (if (<= _returnvalue 1)
      (bind _returnvalue_2 (Class|GameplayStatics|CreatePlayer -1))
      (if (Utilities|IsValid _returnvalue_2)
        (Development|PrintString (Utilities|GetDisplayName _returnvalue_2))
        (else
          (Variables|Default|SetContinue false)))
      (else
        (Variables|Default|SetContinue false)))))

(event EventBeginPlay
  (Development|PrintString "Entering Lobby")
  (CallFunction|CreatePlayers))

(event EventTick
  (params (DeltaSeconds :type Float%20%28single-precision%29))
  (bind _asinstance_aliens_vsgovernment (Utilities|Casting|CastToInstance_AliensVSGovernment (Game|GetGameInstance)))
  (bind _team (Default|FindPlayerConfig _asinstance_aliens_vsgovernment))
  (bind _team_2 (Default|FindPlayerConfig _asinstance_aliens_vsgovernment))
  (Variables|/Game/Blueprints/GameInstance/Instance_AliensVSGovernment.Instance_AliensVSGovernment_C|SetPlayersReady _asinstance_aliens_vsgovernment (and (Utilities|Enum|NotEqual(Enum) _team_2 "NewEnumerator2") (Utilities|Enum|NotEqual(Enum) _team "NewEnumerator2"))))

(fn ConstructionScript)