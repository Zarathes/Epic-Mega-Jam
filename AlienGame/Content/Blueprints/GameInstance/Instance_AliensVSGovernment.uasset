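; Game instance for Aliens vs Government that runs the mini-game flow and keeps the follower score and team assignments.
; StartMiniGame shows a loading screen widget for the selected mini-game, and LoadLevel opens its level.
; WinMiniGame clears widgets, shows the winner screen and shifts one shared follower count up for Aliens or down for Government.
; A map links controller IDs to teams, creating Invalid entries on lookup and backing team availability checks.
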(fn AdjustFollowers
  (params (WinningTeam :type Enum_Teams%20Enum :default "NewEnumerator0"))
  (switch Utilities|FlowControl|Switch|SwitchonEnum_Teams WinningTeam
    (:NewEnumerator0
      (Variables|Score|SetFollowers (+ (Variables|Score|GetFollowers) (* (Variables|Score|GetBaseFollowerChange) (Variables|Score|GetMultiplierFollowerChange)))))
    (:NewEnumerator1
      (Variables|Score|SetFollowers (- (Variables|Score|GetFollowers) (* (Variables|Score|GetBaseFollowerChange) (Variables|Score|GetMultiplierFollowerChange))))))
  (Development|PrintString (Utilities|String|ToString(Integer) (Variables|Score|GetFollowers)))
  (return))

(fn StartMiniGame
  (params (SelectedMiniGame :type Struct%20Mini%20Games%20Structure))
  (bind _returnvalue (UserInterface|CreateWidget "/Game/Blueprints/UI/LoadingScreen/UI_LoadingScreen.UI_LoadingScreen_C" (Game|GetPlayerController 0) SelectedMiniGame))
  (UserInterface|Viewport|AddtoViewport _returnvalue 0)
  (Default|StartMiniGame _returnvalue SelectedMiniGame))

(fn WinMiniGame
  (params (WinningTeam :type Enum_Teams%20Enum :default "NewEnumerator0"))
  (Viewport|RemoveAllWidgets)
  (switch Utilities|FlowControl|Switch|SwitchonEnum_Teams WinningTeam
    (:NewEnumerator0
      (bind _returnvalue (UserInterface|CreateWidget "/Game/Blueprints/UI/MiniGameWonScreen/UI_MiniGameWon.UI_MiniGameWon_C" (Game|GetPlayerController 0)))
      (UserInterface|Viewport|AddtoViewport _returnvalue 0)
      (CallFunction|AdjustFollowers "NewEnumerator0"))
    (:NewEnumerator1
      (bind _returnvalue_2 (UserInterface|CreateWidget "/Game/Blueprints/UI/MiniGameWonScreen/UI_MiniGameWon.UI_MiniGameWon_C" (Game|GetPlayerController 0) "NewEnumerator1"))
      (UserInterface|Viewport|AddtoViewport _returnvalue_2 0)
      (CallFunction|AdjustFollowers "NewEnumerator1"))))

(fn CreatePlayerConfig
  (params (ControllerID :type Integer))
  (Utilities|Map|Add (Variables|Configuration|GetPlayerConfiguration) ControllerID "NewEnumerator2")
  (return "NewEnumerator2"))

(fn FindPlayerConfig
  (params (ControllerID :type Integer))
  (bind _playerconfiguration (Variables|Configuration|GetPlayerConfiguration))
  (bind (_value _returnvalue) (Utilities|Map|Find _playerconfiguration ControllerID))
  (if _returnvalue
    (return _value)
    (else
      (bind _team (CallFunction|CreatePlayerConfig ControllerID))
      (return _team))))

(fn SetPlayerConfig
  (params (ControllerID :type Integer) (Team :type Enum_Teams%20Enum :default "NewEnumerator0"))
  (CallFunction|FindPlayerConfig ControllerID)
  (Utilities|Map|Add (Variables|Configuration|GetPlayerConfiguration) ControllerID Team))

(fn TeamAvailable
  (params (Team :type Enum_Teams%20Enum :default "NewEnumerator0"))
  (bind _values (Utilities|Map|Values (Variables|Configuration|GetPlayerConfiguration)))
  (return (not (Utilities|Array|ContainsItem _values Team))))

(fn LoadLevel
  (params (SelectedMiniGame :type Struct%20Mini%20Games%20Structure))
  (Game|OpenLevel(byName) (.Level (Utilities|Struct|BreakStruct_MiniGames SelectedMiniGame))))